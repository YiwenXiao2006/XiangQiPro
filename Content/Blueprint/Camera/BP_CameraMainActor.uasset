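; BP_CameraMainActor is a main camera Blueprint that eases its offsets toward a preset framing when the game starts from a touch.
; The TouchtoStartGame event sets ClickToStart, after which Tick uses FInterpTo to move RotationZOffset and the Y and Z of LocationOffset toward fixed targets, leaving X unchanged.
; The graph only updates these offset variables and does not itself apply them to a transform.
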(event `self.ReceiveTick`
  (params (DeltaSeconds :type "Float (single-precision)"))
  (bind (_locationoffset_x _locationoffset_y _locationoffset_z) (`KismetMathLibrary.BreakVector` (`self.LocationOffset`)))
  (if (`self.ClickToStart`)
    (set `self.RotationZOffset` (`KismetMathLibrary.FInterpTo` (`self.RotationZOffset`) -10.0 DeltaSeconds 1.5))
    (set `self.LocationOffset` (`KismetMathLibrary.MakeVector` _locationoffset_x (`KismetMathLibrary.FInterpTo` _locationoffset_y 5.906762 DeltaSeconds 1.5) (`KismetMathLibrary.FInterpTo` _locationoffset_z 0.0 DeltaSeconds 1.5)))))

(event `/Game/Blueprint/MainMapInterface.TouchToStartGame`
  (set `self.ClickToStart` true))

(fn `UserConstructionScript`)